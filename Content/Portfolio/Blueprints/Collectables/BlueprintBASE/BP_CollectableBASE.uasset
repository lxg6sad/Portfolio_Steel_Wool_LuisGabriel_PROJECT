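; BP_CollectableBASE is a base Blueprint for collectables, with its appearance driven by variables.
; The construction script applies the mesh, world rotation, world scale and slot 0 material to its StaticMesh component.
; It also assigns CollectableID to itself, and the file shows no pickup logic.
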(fn `UserConstructionScript`
  (`StaticMeshComponent.SetStaticMesh` (`self.StaticMesh`) (`self.Mesh`))
  (`SceneComponent.K2_SetWorldRotation` (`self.StaticMesh`) (`self.MeshRotation`) false false)
  (`SceneComponent.SetWorldScale3D` (`self.StaticMesh`) (`self.MeshScale`))
  (set `self.Collectable ID` (`self.Collectable ID`))
  (`PrimitiveComponent.SetMaterial` (`self.StaticMesh`) 0 (`self.MeshMATERIAL`)))