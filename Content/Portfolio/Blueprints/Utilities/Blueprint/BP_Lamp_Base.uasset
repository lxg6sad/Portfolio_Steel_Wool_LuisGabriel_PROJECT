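; BP_Lamp_Base is a base lamp Blueprint with a spot light that can be switched on and off.
; The Construction Script applies the intensity, color and initial off state from its variables to the SpotLight.
; The AllLIGHTSOFF and AllLIGHTSON events switch the light by toggling its hidden-in-game flag, without propagating to child components or updating LampIsOFF.
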(event `AllLIGHTSOFF`
  (`SceneComponent.SetHiddenInGame` (`self.SpotLight`) true false))

(event `AllLIGHTSON`
  (`SceneComponent.SetHiddenInGame` (`self.SpotLight`) false false))

(fn `UserConstructionScript`
  (bind _spotlight (`self.SpotLight`))
  (`LightComponent.SetIntensity` _spotlight (`self.LampIntensity`))
  (`LightComponent.SetLightColor` _spotlight (`self.LampColor`) true)
  (`SceneComponent.SetHiddenInGame` (`self.SpotLight`) (`self.LampIsOFF?`) true))