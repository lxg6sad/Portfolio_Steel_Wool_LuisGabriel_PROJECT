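; Generator mission objective that the player switches on, with a point light showing its status.
; BeginPlay caches the player and game mode, and the PlayerHIT event, during an active generator mission, fires once to trigger the game mode's message and set GeneratorON.
; Tick re-applies the light color every frame: red while the mission is active and the generator is off, green otherwise, including when no mission is running.
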(event `self.ReceiveBeginPlay`
  ;[1 1 1] CASTS
  (bind _asbp_player (cast `/Game/Portfolio/Blueprints/Player/Blueprints/BP_Player` (`GameplayStatics.GetPlayerCharacter` 0)))
  (set `self.As BP Player` _asbp_player)
  (bind _asbp_game_mode (cast `/Game/Portfolio/Blueprints/Player/Blueprints/BP_GameMODE` (`GameplayStatics.GetGameMode`)))
  (set `self.As BP Game MODE` _asbp_game_mode))

(event `PlayerHIT`
  ;[1 1 1] PlayerHIT
  (if (`/Game/Portfolio/Blueprints/Player/Blueprints/BP_GameMODE.GeneratorMissionON?` (`self.As BP Game MODE`))
    (`/Engine/EditorBlueprintResources/StandardMacros.DoOnce` false
      (:`Completed`
        (message `/Game/Portfolio/Blueprints/Player/Blueprints/BP_PlayerInteractions.Interaction_GeneratorON` (`self.As BP Game MODE`))
        (set `self.GeneratorON?` true)
        (`KismetSystemLibrary.Delay` 0.2)
        (`LightComponent.SetLightColor` (`self.PointLight`) (struct :`R` 0.106598 :`G` 1.0 :`A` 1.0) true)))))

(event `self.ReceiveTick`
  (params (DeltaSeconds :type "Float (single-precision)"))
  (if (`/Game/Portfolio/Blueprints/Player/Blueprints/BP_GameMODE.GeneratorMissionON?` (`self.As BP Game MODE`))
    (if (`self.GeneratorON?`)
      (`LightComponent.SetLightColor` (`self.PointLight`) (struct :`R` 0.005 :`G` 1.0 :`A` 1.0) true :!label _label)
      (else
        (`LightComponent.SetLightColor` (`self.PointLight`) (struct :`R` 1.0 :`A` 1.0) true)))
    (else
      (goto _label))))

(fn `UserConstructionScript`)