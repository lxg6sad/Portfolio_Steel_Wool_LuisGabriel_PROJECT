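; Base enemy AI character that wanders, chases sighted pawns and triggers the player's jumpscare on reaching its target.
; StartMOVEIA enables behavior flags and starts random-point AIMoveTo roaming.
; PawnSensing starts the chase, while a self-recalling delayed event ramps up walk speed.
; A retriggerable delay returns it to roaming after a give-up time and re-arms the DoOnce spotted sound.
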(event `self.ReceiveBeginPlay`
  ;[0.4721 1 0] Cast to player
  (bind _asbp_player (cast `/Game/Portfolio/Blueprints/Player/Blueprints/BP_Player` (`GameplayStatics.GetPlayerCharacter` 0)))
  (set `self.As BP Player` _asbp_player))

(event `MoveRandom`
  ;[0 1 0.9881] IARandomMOVE
  (if (`self.IAMoveRandom?`)
    (`self.SetMaxWalkSpeed` 300.0)
    (set `self.IARunningPLAYER?` false)
    (`|AIMoveTo` self (`NavigationSystemV1.K2_GetRandomReachablePointInRadius` (`SceneComponent.K2_GetComponentLocation` (`self.Cylinder`)) (`self.IAMoveRadius`) null null) null
      (:`OnSuccess`
        _)
      (:`OnFail`
        _))
    (if (`self.IAContinuosMOVE?`)
      (`self.MoveRandom`))))

(event `UpdateRunPLAYER`
  ;[0 0.001623 1] MoreSPEED IA
  (`self.SetMaxWalkSpeed` (`self.IAMaxWALKRunPLAYER`))
  (`KismetSystemLibrary.RetriggerableDelay` 0.1)
  (if (`self.IARunningPLAYER?`) :!label _label
    (`KismetSystemLibrary.Delay` 1.5)
    (set `self.IAMaxWALKRunPLAYER` (+ (`self.IAMaxWALKRunPLAYER`) (`self.IAMoreSPEED`)))
    (else
      (set `self.IAMaxWALKRunPLAYER` (`self.IADefaultRUNPLAYER`))))
  (`self.UpdateRunPLAYER`))

(event `RunPlayer`
  ;[0 0.001623 1] MoreSPEED IA
  (goto _label))

(event `IAJumpScare`
  (bind _as_bp_player (`self.As BP Player`))
  ;[1 0 0] JumpScare
  (if (`/Game/Portfolio/Blueprints/Player/Blueprints/BP_Player.JumpScare ON?` _as_bp_player)
    (`/Game/Portfolio/Blueprints/Player/Blueprints/BP_Player.JumpScare` _as_bp_player)
    (`SceneComponent.SetHiddenInGame` (`self.Cylinder`) true false)
    (else
      (`self.MoveRandom`))))

(event `self.PawnSensing.OnSeePawn`
  (params (Pawn :type "Pawn Object Reference"))
  ;[1 0 0.7133] RunToPlayer
  (if (`self.IARunToPLAYER?`)
    (`|ExecutionSequence`
      (:`then_0`
        (set `self.IARunningPLAYER?` true)
        (`self.SetMaxWalkSpeed` (`self.IAMaxWALKRunPLAYER`))
        (`self.RunPlayer`)
        (`|AIMoveTo` self (0.0 0.0 0.0) Pawn
          (:`OnSuccess`
            (set `self.IARunningPLAYER?` false)
            (`self.IAJumpScare`))
          (:`OnFail`
            (if (`self.IARunningPLAYER?`)
              (`self.MoveRandom`)))))
      (:`then_1`
        (`KismetSystemLibrary.RetriggerableDelay` (`self.IATimeToGiveUP`))
        (`self.MoveRandom`)
        (goto _label_2 :!via `Reset`))
      (:`then_2`
        (`/Engine/EditorBlueprintResources/StandardMacros.DoOnce` false :!label _label_2
          (:`Completed`
            (`GameplayStatics.PlaySound2D` "/Game/Portfolio/Blueprints/IA/Sounds/BotFindsPlayer.BotFindsPlayer" 1.0 1.0 0.0 null null)))))
    (else
      (`self.MoveRandom`))))

(event `StartMOVEIA`
  (set `self.IAContinuosMOVE?` true)
  (set `self.IARunToPLAYER?` true)
  (set `self.IAMoveRandom?` true)
  (`self.MoveRandom`))

(fn `UserConstructionScript`)