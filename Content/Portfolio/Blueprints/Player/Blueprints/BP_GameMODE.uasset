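; Game mode that runs the level's linear mission flow and shows each step through an objective widget created at BeginPlay.
; Collecting the flashlight switches off all lamps and starts a five-generator counter; completing it restores the lights.
; After a delay, the card search begins, starting movement on all AI actors and making the existing card collectable.
; An end trigger collision disables player input and shows the end-game widget.
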(event `self.ReceiveBeginPlay`
  ;[1 0 0] EventBEGINPLAY
  (bind _asbp_player (cast `/Game/Portfolio/Blueprints/Player/Blueprints/BP_Player` (`GameplayStatics.GetPlayerCharacter` 0)))
  (set `self.As BP Player` _asbp_player)
  (bind _returnvalue (`|CreateWidget` "/Game/Portfolio/Blueprints/Player/Widgets/WID_objective.WID_objective_C"))
  (set `self.ObjectivesREF` _returnvalue)
  (`UserWidget.AddToViewport` _returnvalue 0)
  (bind _aswid_objective (cast `/Game/Portfolio/Blueprints/Player/Widgets/WID_objective` (`self.ObjectivesREF`)))
  (set `self.As WID Objective` _aswid_objective))

(event `/Game/Portfolio/Blueprints/Player/Blueprints/BP_PlayerInteractions. Interaction_FlashLIGHTCollected`
  ;[0 1 0.1395] GeneratorMISSION
  ;;[1 1 1] Start Turn ON Generatos
  (`/Game/Portfolio/Blueprints/Player/Widgets/WID_objective.NewObjectives` (`self.As WID Objective`) true (`KismetTextLibrary.Conv_StringToText` (`KismetStringLibrary.Concat_StrStr` "Turn on the generators" " " (`KismetStringLibrary.Conv_IntToString` (`self.GeneratorsON`)) "/" "5")) 2.0 8.0)
  (`self.Turn OFF lights`)
  (set `self.GeneratorMissionON?` true))

(event `Turn OFF lights`
  ;[0 1 0.1395] GeneratorMISSION
  ;;[1 1 1] TurnOFFLights
  (bind _outactors (`GameplayStatics.GetAllActorsOfClass` "/Game/Portfolio/Blueprints/Utilities/Blueprint/BP_Lamp_Base.BP_Lamp_Base_C"))
  (for _array_element _outactors
    (`/Game/Portfolio/Blueprints/Utilities/Blueprint/BP_Lamp_Base.AllLIGHTSOFF` _array_element))
  (`GameplayStatics.PlaySound2D` "/Game/Portfolio/Blueprints/Utilities/Sounds/TurnOFFLights.TurnOFFLights" 1.0 1.0 0.0 null null))

(event `/Game/Portfolio/Blueprints/Player/Blueprints/BP_PlayerInteractions.Interaction_GeneratorON`
  ;[0 1 0.1395] GeneratorMISSION
  ;;[1 1 1] GemeratorON
  (bind _output_get (set `self.GeneratorsON` (`KismetMathLibrary.Clamp` (+ (`self.GeneratorsON`) 1) 0 5)))
  (if (== _output_get 5)
    (bind _outactors (`GameplayStatics.GetAllActorsOfClass` "/Game/Portfolio/Blueprints/Utilities/Blueprint/BP_Lamp_Base.BP_Lamp_Base_C"))
    (for _array_element _outactors
      (`/Game/Portfolio/Blueprints/Utilities/Blueprint/BP_Lamp_Base.AllLIGHTSON` _array_element))
    (`/Engine/EditorBlueprintResources/StandardMacros.DoOnce` false
      (:`Completed`
        (`/Game/Portfolio/Blueprints/Player/Widgets/WID_objective.NewObjectives` (`self.As WID Objective`) true "Turn on the generators COMPLETE" 5.0 8.0)
        (set `self.GeneratorMissionON?` false)
        (`KismetSystemLibrary.Delay` 7.0)
        (`self.GeneratorsCOMPLETE`)))
    (else
      (`/Game/Portfolio/Blueprints/Player/Widgets/WID_objective.NewObjectives` (`self.As WID Objective`) true (`KismetTextLibrary.Conv_StringToText` (`KismetStringLibrary.Concat_StrStr` "Turn on the generators" " " (`KismetStringLibrary.Conv_IntToString` (`self.GeneratorsON`)) "/" "5")) 2.0 8.0))))

(event `GeneratorsCOMPLETE`
  ;[0 1 0.1395] GeneratorMISSION
  ;;[1 1 1] GeneratorsCOMPLETE
  (if (not (`self.GeneratorMissionON?`))
    (`self.StartFIND CARD`)))

(event `StartFIND CARD`
  ;[1 0 0] FindCardMISSION
  ;;[0.2969 0.07886 0.07886] Start FIND card
  (`/Game/Portfolio/Blueprints/Player/Widgets/WID_objective.NewObjectives` (`self.As WID Objective`) true "Search for your card" 6.0 8.0)
  (`KismetSystemLibrary.Delay` 3.0)
  (bind _outactors (`GameplayStatics.GetAllActorsOfClass` "/Game/Portfolio/Blueprints/IA/BP_IA_BASE.BP_IA_BASE_C"))
  (for _array_element _outactors
    (`/Game/Portfolio/Blueprints/IA/BP_IA_BASE.StartMOVEIA` _array_element))
  (`self.Spawn CARD`))

(event `Spawn CARD`
  ;[1 0 0] FindCardMISSION
  ;;[1 0.3646 0.3646] Spawn CARD
  (bind _outactors (`GameplayStatics.GetAllActorsOfClass` "/Game/Portfolio/Blueprints/Collectables/BlueprintBASE/BP_CollectableCARD.BP_CollectableCARD_C"))
  (set `/Game/Portfolio/Blueprints/Collectables/BlueprintBASE/BP_CollectableBASE.IsCollectable?` true (`|GetArrayItem` _outactors)))

(event `/Game/Portfolio/Blueprints/Player/Blueprints/BP_PlayerInteractions.Interaction_TriggerCollision`
  (params (CollisionID :type String))
  ;[1 0 0] FindCardMISSION
  (if (`KismetStringLibrary.EqualEqual_StrStr` CollisionID "END0")
    (`KismetSystemLibrary.PrintString` "2")
    (`self.DisableInput` (`self.As BP Player`) (`GameplayStatics.GetPlayerController` 0))
    (bind _returnvalue (`|CreateWidget` "/Game/Portfolio/Blueprints/Player/Widgets/WID_ENDGAME.WID_ENDGAME_C"))
    (`UserWidget.AddToViewport` _returnvalue 0)
    (else
      (`KismetSystemLibrary.PrintString` "1"))))

(fn `UserConstructionScript`)